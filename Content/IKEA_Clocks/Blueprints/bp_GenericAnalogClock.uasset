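; Generic analog clock actor that shows either computer time or a custom time, with an optional sound alarm.
; A pausable one-second looping timer updates or increments the time, then SetTime rotates the three hands, with fractional hour and minute movement.
; A DoOnce plays the 2D alarm for a set duration when hour and minute match.
; The construction script applies body and dial colours through a dynamic material and previews the hands.
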(event Custom|StartClock
  (bind _returnvalue (Math|DateTime|Now))
  (bind _returnvalue_2 (Math|DateTime|Now))
  (if (Variables|InitialTime|GetUseLocalTime?)
    (Variables|Default|SetYear (.year _returnvalue_2))
    (Variables|Default|SetMonth (.month _returnvalue_2))
    (Variables|Default|SetDate (.day _returnvalue_2))
    (Variables|InitialTime|SetHours (.hour _returnvalue_2))
    (Variables|InitialTime|SetMinutes (.minute _returnvalue_2))
    (Variables|InitialTime|SetSeconds (.second _returnvalue_2))
    (else
      (Variables|Default|SetYear (.year (+ (Math|DateTime|MakeDateTime (.year _returnvalue) (.month _returnvalue) (.day _returnvalue) (Variables|InitialTime|GetHours) (Variables|InitialTime|GetMinutes) (Variables|InitialTime|GetSeconds)) (Math|Timespan|MakeTimespan 0 0 0 1))))
      (Variables|Default|SetMonth (.month (+ (Math|DateTime|MakeDateTime (.year _returnvalue) (.month _returnvalue) (.day _returnvalue) (Variables|InitialTime|GetHours) (Variables|InitialTime|GetMinutes) (Variables|InitialTime|GetSeconds)) (Math|Timespan|MakeTimespan 0 0 0 1))))
      (Variables|Default|SetDate (.day (+ (Math|DateTime|MakeDateTime (.year _returnvalue) (.month _returnvalue) (.day _returnvalue) (Variables|InitialTime|GetHours) (Variables|InitialTime|GetMinutes) (Variables|InitialTime|GetSeconds)) (Math|Timespan|MakeTimespan 0 0 0 1))))
      (Variables|InitialTime|SetHours (.hour (+ (Math|DateTime|MakeDateTime (.year _returnvalue) (.month _returnvalue) (.day _returnvalue) (Variables|InitialTime|GetHours) (Variables|InitialTime|GetMinutes) (Variables|InitialTime|GetSeconds)) (Math|Timespan|MakeTimespan 0 0 0 1))))
      (Variables|InitialTime|SetMinutes (.minute (+ (Math|DateTime|MakeDateTime (.year _returnvalue) (.month _returnvalue) (.day _returnvalue) (Variables|InitialTime|GetHours) (Variables|InitialTime|GetMinutes) (Variables|InitialTime|GetSeconds)) (Math|Timespan|MakeTimespan 0 0 0 1))))
      (Variables|InitialTime|SetSeconds (.second (+ (Math|DateTime|MakeDateTime (.year _returnvalue) (.month _returnvalue) (.day _returnvalue) (Variables|InitialTime|GetHours) (Variables|InitialTime|GetMinutes) (Variables|InitialTime|GetSeconds)) (Math|Timespan|MakeTimespan 0 0 0 1))))))
  (CallFunction|SetTime)
  (if (Variables|SetAlarm|GetAlarm)
    (if (and (== (Variables|SetAlarm|GetAlarm%20Minutes) (Variables|InitialTime|GetMinutes)) (== (Variables|SetAlarm|GetAlarm%20Hours) (Variables|InitialTime|GetHours)))
      (Utilities|FlowControl|DoOnce false :!label _label
        (:Completed
          (CallFunction|PlayAlarmSound)
          (Utilities|FlowControl|Delay (Variables|SetAlarm|GetAlarm%20Longevity%20sec))
          (CallFunction|StopAlarmSound)))
      (else
        (goto _label Reset)))))

(event Custom|SetAndStartClock
  (params (LocalComputerTime? :type Boolean) (NewTime :type Date%20Time%20Structure))
  (bind _returnvalue (Math|DateTime|Now))
  (if LocalComputerTime?
    (Variables|InitialTime|SetUseLocalTime? LocalComputerTime?)
    (Variables|Default|SetYear (.year _returnvalue))
    (Variables|Default|SetMonth (.month _returnvalue))
    (Variables|Default|SetDate (.day _returnvalue))
    (Variables|InitialTime|SetHours (.hour _returnvalue))
    (Variables|InitialTime|SetMinutes (.minute _returnvalue))
    (Variables|InitialTime|SetSeconds (.second _returnvalue))
    (CallFunction|SetTime)
    (Utilities|Time|UnpauseTimerbyHandle (Variables|Default|GetTimer))
    (else
      (Variables|InitialTime|SetUseLocalTime? false)
      (Variables|Default|SetYear (.year NewTime))
      (Variables|Default|SetMonth (.month NewTime))
      (Variables|Default|SetDate (.day NewTime))
      (Variables|InitialTime|SetHours (.hour NewTime))
      (Variables|InitialTime|SetMinutes (.minute NewTime))
      (Variables|InitialTime|SetSeconds (.second NewTime))
      (Utilities|Time|UnpauseTimerbyHandle (Variables|Default|GetTimer)))))

(event Custom|StopClock
  (Utilities|Time|PauseTimerbyHandle (Variables|Default|GetTimer)))

(event EventBeginPlay
  (bind _returnvalue (Math|DateTime|Now))
  (bind _returnvalue_2 (Utilities|Time|SetTimerbyEvent (delegate Custom|StartClock) 1.0 true))
  (bind _output_get (Variables|Default|SetTimer _returnvalue_2))
  (Utilities|Time|PauseTimerbyHandle _output_get)
  (Variables|Default|SetYear (.year _returnvalue))
  (Variables|Default|SetMonth (.month _returnvalue))
  (Variables|Default|SetDate (.day _returnvalue))
  (if (not (Variables|InitialTime|GetManualStart?))
    (CallFunction|SetandStartClock (Variables|InitialTime|GetUseLocalTime?))))

(fn ConstructionScript
  (bind _returnvalue (Math|DateTime|Now))
  (bind (_year _month _day) (Math|DateTime|BreakDateTime _returnvalue))
  (bind _returnvalue_2 (Rendering|Material|CreateDynamicMaterialInstance (Variables|Default|GetBody) 0 (Rendering|Material|GetMaterial (Variables|Default|GetBody) 0) "None" :!class /Script/Engine.PrimitiveComponent))
  (Variables|Material|SetMaterialInstance _returnvalue_2)
  (Rendering|Material|SetVectorParameterValue _returnvalue_2 "Colour1" (Variables|Material|GetBody%20Colour) :!class /Script/Engine.MaterialInstanceDynamic)
  (Rendering|Material|SetVectorParameterValue _returnvalue_2 "Colour2" (Variables|Material|GetDial%20Colour) :!class /Script/Engine.MaterialInstanceDynamic)
  (Rendering|Material|SetMaterial (Variables|Default|GetSecondsHand) 0 (Variables|Material|GetMaterialInstance))
  (Rendering|Material|SetMaterial (Variables|Default|GetHourHand) 0 (Variables|Material|GetMaterialInstance))
  (Rendering|Material|SetMaterial (Variables|Default|GetMinuteHand) 0 (Variables|Material|GetMaterialInstance))
  (Variables|Default|SetYear (.year (select (Variables|InitialTime|GetUseLocalTime?) _returnvalue (Math|DateTime|MakeDateTime _year _month _day (Variables|InitialTime|GetHours) (Variables|InitialTime|GetMinutes) (Variables|InitialTime|GetSeconds) 11))))
  (Variables|Default|SetMonth (.month (select (Variables|InitialTime|GetUseLocalTime?) _returnvalue (Math|DateTime|MakeDateTime _year _month _day (Variables|InitialTime|GetHours) (Variables|InitialTime|GetMinutes) (Variables|InitialTime|GetSeconds) 11))))
  (Variables|Default|SetDate (.day (select (Variables|InitialTime|GetUseLocalTime?) _returnvalue (Math|DateTime|MakeDateTime _year _month _day (Variables|InitialTime|GetHours) (Variables|InitialTime|GetMinutes) (Variables|InitialTime|GetSeconds) 11))))
  (Variables|InitialTime|SetHours (.hour (select (Variables|InitialTime|GetUseLocalTime?) _returnvalue (Math|DateTime|MakeDateTime _year _month _day (Variables|InitialTime|GetHours) (Variables|InitialTime|GetMinutes) (Variables|InitialTime|GetSeconds) 11))))
  (Variables|InitialTime|SetMinutes (.minute (select (Variables|InitialTime|GetUseLocalTime?) _returnvalue (Math|DateTime|MakeDateTime _year _month _day (Variables|InitialTime|GetHours) (Variables|InitialTime|GetMinutes) (Variables|InitialTime|GetSeconds) 11))))
  (Variables|InitialTime|SetSeconds (.second (select (Variables|InitialTime|GetUseLocalTime?) _returnvalue (Math|DateTime|MakeDateTime _year _month _day (Variables|InitialTime|GetHours) (Variables|InitialTime|GetMinutes) (Variables|InitialTime|GetSeconds) 11))))
  (CallFunction|SetTime))

(fn SetTime
  (bind _minutes (Variables|InitialTime|GetMinutes))
  (Transformation|SetRelativeRotation (Variables|Default|GetHourHand) (Math|Rotator|MakeRotator 0.0 (Math|Float|MapRangeClamped (+ (Math|Conversions|ToFloat(Integer) (Math|Integer|%(Integer) (Variables|InitialTime|GetHours) 12)) (Math|Float|MapRangeClamped (Math|Conversions|ToFloat(Integer) _minutes) 0.0 6e+01 0.0 1.0)) 0.0 12.0 3.6e+02 0.0) 0.0) false false)
  (Transformation|SetRelativeRotation (Variables|Default|GetMinuteHand) (Math|Rotator|MakeRotator 0.0 (Math|Float|MapRangeClamped (+ (Math|Conversions|ToFloat(Integer) (Math|Integer|%(Integer) _minutes 60)) (Math|Float|MapRangeClamped (Math|Conversions|ToFloat(Integer) (Variables|InitialTime|GetSeconds)) 0.0 6e+01 0.0 1.0)) 0.0 6e+01 3.6e+02 0.0) 0.0) false false)
  (Transformation|SetRelativeRotation (Variables|Default|GetSecondsHand) (Math|Rotator|MakeRotator 0.0 (Math|Float|MapRangeClamped (Math|Conversions|ToFloat(Integer) (Math|Integer|%(Integer) (Variables|InitialTime|GetSeconds) 60)) 0.0 6e+01 3.6e+02 0.0) 0.0) false false))

(fn PlayAlarmSound
  (bind _soundalarm (Variables|SetAlarm|GetSoundAlarm)
    (:then
      (bind _returnvalue (Audio|CreateSound2D _soundalarm 1.0 1.0 0.0 0 false false))
      (bind _output_get (Variables|Default|SetAlarmComponent _returnvalue))
      (Audio|Components|Audio|Play _output_get 0.0))
    (:else)))

(fn GetClockTime
  (return (Math|DateTime|MakeDateTime (Variables|Default|GetYear) (Variables|Default|GetMonth) (Variables|Default|GetDate) (Variables|InitialTime|GetHours) (Variables|InitialTime|GetMinutes) (Variables|InitialTime|GetSeconds) 0)))

(fn StopAlarmSound
  (bind _alarmcomponent (Variables|Default|GetAlarmComponent)
    (:then
      (if (Audio|Components|Audio|IsPlaying _alarmcomponent)
        (Audio|Components|Audio|Stop _alarmcomponent)
        (Components|DestroyComponent (Variables|Default|GetAlarmComponent))))
    (:else)))